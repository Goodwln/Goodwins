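; BP_DeadAICharacter is a stand-in corpse for an AI character, turning a copy of its mesh into a ragdoll.
; DeathDescription takes the character's mesh, offsets its own skeletal mesh by that mesh's origin transform, then copies the skeletal mesh and every material.
; It then applies the Ragdoll collision profile and enables physics simulation.
; The event graph and construction script are empty.
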(event EventBeginPlay)

(event Collision|EventActorBeginOverlap
  (params (OtherActor :type Actor%20Object%20Reference)))

(event EventTick
  (params (DeltaSeconds :type Float%20%28single-precision%29)))

(fn ConstructionScript)

(fn DeathDescription
  (params (Mesh :type Skeletal%20Mesh%20Component%20Object%20Reference))
  (bind _output_get (Variables|Default|SetAICharacterMesh Mesh))
  (bind _returnvalue (Class|MovieSceneTransformOrigin|GetTransformOrigin(Message) _output_get))
  (Class|SceneComponent|AddWorldTransform (Variables|Default|GetSkeletalMesh) _returnvalue false false)
  (Class|SkinnedMeshComponent|SetSkeletalMesh (Variables|Default|GetSkeletalMesh) (Variables|/Script/Engine.SkinnedMeshComponent|GetSkeletalMesh (Variables|Default|GetAICharacterMesh)) false)
  (for (_array_element _array_index) (Rendering|Material|GetMaterials (Variables|Default|GetAICharacterMesh))
    (Rendering|Material|SetMaterial (Variables|Default|GetSkeletalMesh) _array_index _array_element))
  (Collision|SetCollisionProfileName (Variables|Default|GetSkeletalMesh) "Ragdoll" true :!class /Script/Engine.PrimitiveComponent)
  (Physics|SetSimulatePhysics (Variables|Default|GetSkeletalMesh) true))