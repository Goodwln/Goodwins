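; Player character Blueprint that adjusts the camera spring arm length while the player sprints.
; BeginPlay caches the default arm length and the Box component's scaled extent.
; Sprint start plays a timeline that lerps the arm from its default toward the sprint length, and sprint end reverses that timeline to ease it back.
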(event EventOnSprintEnd
  (bind _newtrack_0 (Timeline|SprintArmSprintTimeline Reverse)
    (:Update
      (Variables|/Script/Engine.SpringArmComponent|SetTargetArmLength (Variables|Default|GetSpringArmComponent) (Math|Float|Lerp (Variables|SpringSettings|GetDefaultArmLength) (Variables|SpringSettings|GetSpringArmLength) _newtrack_0)))))

(event EventOnSprintStart
  (bind _newtrack_0 (Timeline|SprintArmSprintTimeline Play)
    (:Update
      (Variables|/Script/Engine.SpringArmComponent|SetTargetArmLength (Variables|Default|GetSpringArmComponent) (Math|Float|Lerp (Variables|SpringSettings|GetDefaultArmLength) (Variables|SpringSettings|GetSpringArmLength) _newtrack_0)))))

(event EventBeginPlay
  (Variables|SpringSettings|SetDefaultArmLength (Variables|/Script/Engine.SpringArmComponent|GetTargetArmLength (Variables|Default|GetSpringArmComponent)))
  (Variables|Default|SetBoxExtern (Components|Box|GetScaledBoxExtent (Variables|Default|GetBox))))

(fn ConstructionScript)