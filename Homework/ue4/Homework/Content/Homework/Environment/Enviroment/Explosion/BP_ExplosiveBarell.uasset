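; BP_ExplosiveBarell is an explosive barrel actor that detonates when it takes any damage.
; On BeginPlay it binds to its damage event, which triggers the Explode call on its Explosion component.
; When that component reports the explosion, the barrel hides its Cylinder mesh, disables its collision and sets a five-second lifespan before removal.
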(event OnExplosion(Explosion)
  (CallFunction|ActorDestroy))

(event Custom|OnDamageRecieved
  (params (DamagedActor :type Actor%20Object%20Reference) (Damage :type Float%20%28single-precision%29) (DamageType :type Damage%20Type%20Object%20Reference) (InstigatedBy :type Controller%20Object%20Reference) (DamageCauser :type Actor%20Object%20Reference))
  (Class|ExplosionComponent|Explode (Variables|Default|GetExplosion)))

(event EventBeginPlay
  (EventDispatchers|BindEventtoOnTakeAnyDamage (delegate Custom|OnDamageRecieved)))

(fn ConstructionScript)

(fn ActorDestroy
  (Rendering|SetVisibility (Variables|Default|GetCylinder) false false)
  (Collision|SetCollisionEnabled (Variables|Default|GetCylinder) "NoCollision")
  (Actor|SetLifeSpan 5.0))